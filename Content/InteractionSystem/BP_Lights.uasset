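; BP_Lights is an interactable lights Blueprint that switches three spotlights on or off according to the referenced character's HasFuse flag.
; Interact inverts HasFuse on the character itself, then applies the new value as the visibility of all three spotlights.
; The construction script applies the same flag to set their initial visibility.
; GetInfos is an empty stub.
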(event EventBeginPlay)

(event EventInteract
  (bind _characterref (Variables|Default|GetCharacterRef))
  (bind _output_get (Variables|/Game/FirstPersonCharacter.FirstPersonCharacter_C|SethasFuse? _characterref (not (Variables|/Game/FirstPersonCharacter.FirstPersonCharacter_C|GethasFuse? _characterref))))
  (Rendering|SetVisibility (Variables|Default|GetSpotLight1) _output_get false))

(fn ConstructionScript
  (Rendering|SetVisibility (Variables|Default|GetSpotLight1) (Variables|/Game/FirstPersonCharacter.FirstPersonCharacter_C|GethasFuse? (Variables|Default|GetCharacterRef)) false))

(fn GetInfos
  (params (ObjectName :type Name :default "None"))
  (return ""))