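; BP_Fuse is an interactable fuse pickup in the interaction system.
; On Interact it calls the parent handler, then casts the stored character reference to FirstPersonCharacter and sets its HasFuse flag.
; It prints an on-screen pickup message and destroys itself.
; GetInfos is an empty override, and the construction script only calls the parent.
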(event EventBeginPlay
  (|CallParentFunction) ; This node is disabled and will not be called.\nDrag off pins to build functionality.
)

(event Collision|EventActorBeginOverlap
  (params (OtherActor :type Actor%20Object%20Reference)))

(event EventTick
  (params (DeltaSeconds :type Float%20%28single-precision%29)))

(event EventInteract
  (|CallParentFunction)
  (bind _asfirst_person_character (Utilities|Casting|CastToFirstPersonCharacter (Variables|Default|GetFirstPersonCharacterRef)))
  (Variables|/Game/FirstPersonCharacter.FirstPersonCharacter_C|SethasFuse? _asfirst_person_character true)
  (Development|PrintString "I HAVE FOUND A FUSE !!!" true true "(R=1.000000,G=0.046319,B=0.000000,A=1.000000)" 5e+01)
  (Actor|DestroyActor))

(fn ConstructionScript
  (|CallParentFunction))

(fn GetInfos
  (params (ObjectName :type Name :default "None"))
  (return ""))