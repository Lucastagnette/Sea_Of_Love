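; BP_Door is an interactable door that moves along Z when the Interact key is pressed near it.
; Overlap with BP_FirstPersonCharacter on CollisionBox enables input and opens a gate, and leaving reverses both.
; A forward-only timeline lerps the door's relative Z from ClosedAngle toward its current world Z plus OpenAngle0, re-read each update.
; A click sound node is present but unconnected.
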(event OnComponentBeginOverlap(CollisionBox)
  (params (OverlappedComponent :type Primitive%20Component%20Object%20Reference) (OtherActor :type Actor%20Object%20Reference) (OtherComp :type Primitive%20Component%20Object%20Reference) (OtherBodyIndex :type Integer) (bFromSweep :type Boolean) (SweepResult :type Hit%20Result%20Structure%20%28by%20ref%29))
  (Utilities|Casting|CastToBP_FirstPersonCharacter OtherActor)
  (Input|EnableInput (Game|GetPlayerController 0))
  (Utilities|FlowControl|Gate true) ; enters at Open
)

(event OnComponentEndOverlap(CollisionBox)
  (params (OverlappedComponent :type Primitive%20Component%20Object%20Reference) (OtherActor :type Actor%20Object%20Reference) (OtherComp :type Primitive%20Component%20Object%20Reference) (OtherBodyIndex :type Integer))
  (Utilities|Casting|CastToBP_FirstPersonCharacter OtherActor)
  (Input|DisableInput (Game|GetPlayerController 0))
  (Utilities|FlowControl|Gate true) ; enters at Close
)

(event Input|ActionEvents|InputActionInteract
  (params (Key :type Key%20Structure :default "None"))
  (:Pressed
    (Utilities|FlowControl|Gate true
      (:Exit
        ;[1 1 1] Close/Open Anim
        (bind _door_track (Timeline|Timeline_0 Play)
          (:Update
            (Transformation|SetRelativeLocation (Variables|Default|GetDoor) (Math|Vector|MakeVector 0.0 0.0 (Math|Float|Lerp (Variables|Default|GetClosed%20Angle) (.z (+ (Transformation|GetWorldLocation (Variables|Default|GetDoor)) (Variables|Default|GetOpen%20Angle_0))) _door_track)) false false)))))))

(fn ConstructionScript)