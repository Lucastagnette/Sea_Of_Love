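; BP_LockedDoor is a door that opens on the Interact input only when the first-person character has a key.
; Its collision box caches the overlapping character, toggles input and opens or closes a gate as the player enters or leaves.
; With a key, a timeline lerps the door's yaw from closed to open angle, with no reverse path; without one, a click sound plays.
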(event OnComponentBeginOverlap(CollisionBox)
  (params (OverlappedComponent :type Primitive%20Component%20Object%20Reference) (OtherActor :type Actor%20Object%20Reference) (OtherComp :type Primitive%20Component%20Object%20Reference) (OtherBodyIndex :type Integer) (bFromSweep :type Boolean) (SweepResult :type Hit%20Result%20Structure%20%28by%20ref%29))
  (bind _asbp_first_person_character (Utilities|Casting|CastToBP_FirstPersonCharacter OtherActor))
  (Input|EnableInput (Game|GetPlayerController 0))
  (Utilities|FlowControl|Gate true) ; enters at Open
)

(event OnComponentEndOverlap(CollisionBox)
  (params (OverlappedComponent :type Primitive%20Component%20Object%20Reference) (OtherActor :type Actor%20Object%20Reference) (OtherComp :type Primitive%20Component%20Object%20Reference) (OtherBodyIndex :type Integer))
  (Utilities|Casting|CastToBP_FirstPersonCharacter OtherActor)
  (Input|DisableInput (Game|GetPlayerController 0))
  (Utilities|FlowControl|Gate true) ; enters at Close
)

(event Input|ActionEvents|InputActionInteract
  (params (Key :type Key%20Structure :default "None"))
  (:Pressed
    (if (Variables|/Game/FirstPerson/Blueprints/BP_FirstPersonCharacter.BP_FirstPersonCharacter_C|GetHasKey? (stale OnComponentBeginOverlap(CollisionBox) _asbp_first_person_character))
      (Utilities|FlowControl|Gate true
        (:Exit
          ;[1 1 1] Close/Open Anim
          (bind _door_track (Timeline|Timeline_0 Play)
            (:Update
              (Transformation|SetRelativeRotation (Variables|Default|GetDoor) (Math|Rotator|MakeRotator 0.0 0.0 (Math|Float|Lerp (Variables|Default|GetClosed%20Angle) (Variables|Default|GetOpen%20Angle_0) _door_track)) false false)))))
      (else
        (Audio|PlaySound2D "/Game/InteractionSystem/Sfx/click3_Cue.click3_Cue" 1.0 1.0 0.0 0 0)))))

(fn ConstructionScript)