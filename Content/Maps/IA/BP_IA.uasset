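; BP_IA is an AI pawn that chases the player once it sees them.
; PawnSensing sets a seeing flag and triggers an AI MoveTo toward the player, which plays a one-time weapon sound at the player's location on success.
; Tick halts movement while the flag is false, but nothing clears the flag once set.
; Point damage is only printed, and the attack itself deals none.
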(event OnSeePawn(PawnSensing)
  (params (Pawn :type Pawn%20Object%20Reference))
  (Variables|Default|SetIsSeeingPlayer true)
  (CallFunction|FollowPlayer))

(event Custom|Follow%20Player
  (bind _returnvalue (Game|GetPlayerCharacter 0))
  (if (Variables|Default|GetIsSeeingPlayer)
    (AI|AIMoveTo self "0, 0, 0" _returnvalue 1e+01 false
      (:OnSuccess
        (if (Variables|Default|Getcan%20Attack%20?)
          (Variables|Default|Setcan%20Attack%20? false)
          (Audio|PlaySoundatLocation "/Game/DetectiveStart/FirstPerson/Audio/FirstPersonTemplateWeaponFire02.FirstPersonTemplateWeaponFire02" (Transformation|GetActorLocation _returnvalue) "0, 0, 0" 1.0 1.0 0.0 0 0 0 0))))
    (else
      (Variables|Default|SetIsSeeingPlayer false))))

(event Game|Damage|EventPointDamage
  (params (Damage :type Float%20%28single-precision%29) (DamageType :type Damage%20Type%20Object%20Reference) (HitLocation :type Vector :default "0, 0, 0") (HitNormal :type Vector :default "0, 0, 0") (HitComponent :type Primitive%20Component%20Object%20Reference) (BoneName :type Name :default "None") (ShotFromDirection :type Vector :default "0, 0, 0") (InstigatedBy :type Controller%20Object%20Reference) (DamageCauser :type Actor%20Object%20Reference) (HitInfo :type Hit%20Result%20Structure%20%28by%20ref%29))
  (Development|PrintString (Utilities|String|ToString(Float) Damage)))

(event EventTick
  (params (DeltaSeconds :type Float%20%28single-precision%29))
  (if (not (Variables|Default|GetIsSeeingPlayer))
    (Components|Movement|StopMovementImmediately (Variables|Character|GetCharacterMovement))))

(fn ConstructionScript)